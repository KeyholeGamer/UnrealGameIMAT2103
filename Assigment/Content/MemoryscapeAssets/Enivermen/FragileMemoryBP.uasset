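; FragileMemoryBP is a fragile surface that breaks when the player character touches it and later restores itself.
; Box begin overlap by ThirdPersonCharacter swaps to a touched material, plays a break sound, then after a short delay hides the static mesh and disables its collision.
; Box end overlap, unfiltered by actor type, waits longer, then plays a return sound and restores material, visibility and collision.
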(event OnComponentBeginOverlap(box)
  (params (OverlappedComponent :type Primitive%20Component%20Object%20Reference) (OtherActor :type Actor%20Object%20Reference) (OtherComp :type Primitive%20Component%20Object%20Reference) (OtherBodyIndex :type Integer) (bFromSweep :type Boolean) (SweepResult :type Hit%20Result%20Structure%20%28by%20ref%29))
  (Utilities|Casting|CastToThirdPersonCharacter OtherActor)
  (Rendering|Material|SetMaterial (Variables|Default|GetStaticMesh) 0 "/Game/MemoryscapeAssets/Materials/FragileTouchedMT1.FragileTouchedMT1")
  (Audio|PlaySoundatLocation "/Game/MemoryscapeAssets/Auido/SoundEffects/FragilBreak.FragilBreak" (Transformation|GetActorLocation) "0, 0, 0" 1.0 1.0 0.0 0 0 0)
  (Utilities|FlowControl|Delay 1.5)
  (Rendering|SetVisibility (Variables|Default|GetStaticMesh) false false)
  (Collision|SetCollisionEnabled (Variables|Default|GetStaticMesh) "NoCollision"))

(event OnComponentEndOverlap(box)
  (params (OverlappedComponent :type Primitive%20Component%20Object%20Reference) (OtherActor :type Actor%20Object%20Reference) (OtherComp :type Primitive%20Component%20Object%20Reference) (OtherBodyIndex :type Integer))
  (Utilities|FlowControl|Delay 3.5)
  (Audio|PlaySoundatLocation "/Game/MemoryscapeAssets/Auido/SoundEffects/FragilReturn.FragilReturn" (Transformation|GetActorLocation) "0, 0, 0" 1.0 1.0 0.0 0 0 0)
  (Rendering|Material|SetMaterial (Variables|Default|GetStaticMesh) 0 "/Game/MemoryscapeAssets/Materials/FragileUntouchedMT.FragileUntouchedMT")
  (Rendering|SetVisibility (Variables|Default|GetStaticMesh) true false)
  (Collision|SetCollisionEnabled (Variables|Default|GetStaticMesh) "QueryAndPhysics"))

(event EventBeginPlay)

(event Collision|EventActorBeginOverlap
  (params (OtherActor :type Actor%20Object%20Reference)))

(event EventTick
  (params (DeltaSeconds :type Float%20%28single-precision%29)))

(fn ConstructionScript)